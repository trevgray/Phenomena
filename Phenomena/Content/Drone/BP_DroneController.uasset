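; BP_DroneController is a controller that lets the player switch between drone characters.
; On BeginPlay it collects every BP_DroneCharacter in the level into an array and possesses the first.
; Three ChangeDrone input actions pass fixed indices to SwitchDrone, which unpossesses the current pawn and possesses the drone at that index.
; The array follows GetAllActorsOfClass order, with no bounds check on the index.
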(event `self.ReceiveBeginPlay`
  (bind _outactors (`GameplayStatics.GetAllActorsOfClass` "/Game/Drone/BP_DroneCharacter.BP_DroneCharacter_C"))
  (set `self.DroneArray` _outactors)
  (`self.SwitchDrone` 0))

(event `InputAction|ChangeDrone1`
  (params (Key :type "Key Structure"))
  (:`Pressed`
    (`self.SwitchDrone` 0)))

(event `InputAction|ChangeDrone2`
  (params (Key :type "Key Structure"))
  (:`Pressed`
    (`self.SwitchDrone` 1)))

(event `InputAction|ChangeDrone3`
  (params (Key :type "Key Structure"))
  (:`Pressed`
    (`self.SwitchDrone` 2)))

(fn `SwitchDrone`
  (params (NewDroneIndex :type Integer))
  (bind _output_get (set `self.DroneIndex` NewDroneIndex))
  (`self.UnPossess`)
  (`self.Possess` (`|GetArrayItem` (`self.DroneArray`) _output_get)))

(fn `UserConstructionScript`)